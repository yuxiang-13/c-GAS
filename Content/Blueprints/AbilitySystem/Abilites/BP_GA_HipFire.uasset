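; Gameplay ability for automatic hip-fire shooting with the equipped weapon, activated from an event.
; It plays the weapon's attack montage, fires immediately and repeats on a looping timer set by fire rate.
; Each shot line-traces from the muzzle using control rotation and applies the weapon's effect spec to hit actors with an ability system.
; An attack-ended event or montage end stops the ability, clearing the timer.
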(event Custom|Shoot
  (bind _returnvalue (Class|GAInventoryAbility|GetEquippedWeaponItemActor))
  (bind _returnvalue_2 (Class|WeaponItemActor|GetMuzzleLocation _returnvalue))
  (bind (_outhit _returnvalue_3) (Collision|LineTraceByChannel _returnvalue_2 (+ _returnvalue_2 (* (Pawn|GetControlRotation (.PlayerController (Utilities|Struct|BreakGameplayAbilityActorInfo (Ability|GetActorInfo))) :!class /Script/Engine.Controller) (Variables|Default|GetShootingDistance))) "TraceTypeQuery2" false 0 "ForDuration"))
  (if _returnvalue_3
    (Utilities|IsValid (Ability|GetAbilitySystemComponent (.HitActor (Collision|BreakHitResult _outhit)))
      (:Is%20Valid
        ;[1 1 1] 应用GE实例
        (GameplayEffects|ApplyGameplayEffectSpecToSelf (Ability|GetAbilitySystemComponent (.HitActor (Collision|BreakHitResult _outhit))) (Class|GAInventoryCombatAbility|GetWeaponEffectSpec _outhit))))))

(event Ability|EventOnEndAbility
  (params (bWasCancelled :type Boolean))
  (Utilities|Time|ClearandInvalidateTimerbyHandle (Variables|Default|GetTimeHandle)))

(event Ability|EventActivateAbilityFromEvent
  (params (EventData :type Gameplay%20Event%20Data%20Structure%20%28by%20ref%29))
  (bind _returnvalue (Class|GAInventoryAbility|GetEquippedItemWeaponStaticData))
  ;[1 1 1] 蒙太奇中合适时机触发GA
  (|PlayMontageandWaitProxy "None" (Variables|/Script/ActionGASProject.WeaponStaticData|GetAttackMontage _returnvalue) 1.0 "None" true 1.0 0.0
    (:then
      (bind _returnvalue_2 (Utilities|Time|SetTimerbyEvent (delegate Custom|Shoot) (/ 1.0 (Variables|/Script/ActionGASProject.WeaponStaticData|GetFireRate _returnvalue)) true))
      (Variables|Default|SetTimeHandle _returnvalue_2)
      (CallFunction|Shoot)
      (Ability|Tasks|WaitGameplayEvent "(TagName=\"Event.Combat.Attack.Ended\")" 0 true
        (:EventReceived
          (Ability|EndAbility))))
    (:OnCompleted
      (Ability|EndAbility :!label _label))
    (:OnInterrupted
      (goto _label))
    (:OnCancelled
      (goto _label))))