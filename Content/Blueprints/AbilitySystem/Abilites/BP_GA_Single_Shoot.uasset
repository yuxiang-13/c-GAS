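; Gameplay ability that fires a single shot from the equipped weapon.
; It plays the weapon's attack montage and waits for an Event.Combat.Shoot gameplay event to time the shot.
; Shoot traces from weapon to focus, plays weapon effects, and applies the weapon's effect spec to any hit actor with an ability system component, printing its name for debug.
; The ability ends after the shot or when the montage completes, is interrupted or cancelled.
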(event Custom|Shoot
  (bind _shootingdistance (Variables|Default|GetShootingDistance))
  (bind (_outhitresult _returnvalue) (Class|GAInventoryCombatAbility|GetWeapontoFocusTraceResult _shootingdistance "TraceTypeQuery3"))
  (bind _hitactor (Collision|BreakHitResult _outhitresult))
  (bind _returnvalue_2 (Ability|GetAbilitySystemComponent _hitactor))
  (Class|WeaponItemActor|PlayWeaponEffects (Class|GAInventoryAbility|GetEquippedWeaponItemActor) _outhitresult)
  (if _returnvalue
    (Utilities|IsValid _returnvalue_2
      (:Is%20Valid
        (Development|PrintString (Utilities|GetDisplayName _hitactor) true true "(R=0.000000,G=0.660000,B=1.000000,A=1.000000)" 1e+01)
        ;[1 1 1] 应用GE实例
        (GameplayEffects|ApplyGameplayEffectSpecToSelf _returnvalue_2 (Class|GAInventoryCombatAbility|GetWeaponEffectSpec _outhitresult)))
      (:Is%20Not%20Valid
        _)))
  (Ability|EndAbility))

(event Ability|EventActivateAbilityFromEvent
  (params (EventData :type Gameplay%20Event%20Data%20Structure%20%28by%20ref%29))
  ;[1 1 1] 蒙太奇中合适时机触发GA
  (|PlayMontageandWaitProxy "None" (Variables|/Script/ActionGASProject.WeaponStaticData|GetAttackMontage (Class|GAInventoryAbility|GetEquippedItemWeaponStaticData)) 1.0 "None" true 1.0 0.0
    (:then
      ;[1 1 1] 开枪之后等待Notify发送时间通知
      (Ability|Tasks|WaitGameplayEvent "(TagName=\"Event.Combat.Shoot\")" 0 true
        (:EventReceived
          ;[1 1 1] 成功接收
          (CallFunction|Shoot))))
    (:OnCompleted
      (Ability|EndAbility :!label _label))
    (:OnInterrupted
      (goto _label))
    (:OnCancelled
      (goto _label))))